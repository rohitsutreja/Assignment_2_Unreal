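; BP_MyPlayerController is a player controller Blueprint that displays attribute values as debug text.
; Its ShowAttributes event receives an Attributes value and prints Health, Stamina and Speed as separate labeled strings through PrintString.
; BeginPlay, Tick and the construction script contain no logic.
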(event `self.ShowAttributes`
  (params (Attributes :type "PawnAttributeAsset Object Reference"))
  (`KismetSystemLibrary.PrintString` (`KismetStringLibrary.Concat_StrStr` "Health: " (`KismetStringLibrary.Conv_DoubleToString` (`PawnAttributeAsset.Health` Attributes))))
  (`KismetSystemLibrary.PrintString` (`KismetStringLibrary.Concat_StrStr` "Stamina: " (`KismetStringLibrary.Conv_DoubleToString` (`PawnAttributeAsset.Stamina` Attributes))))
  (`KismetSystemLibrary.PrintString` (`KismetStringLibrary.Concat_StrStr` "Speed: " (`KismetStringLibrary.Conv_DoubleToString` (`PawnAttributeAsset.Speed` Attributes)))))

(fn `UserConstructionScript`)